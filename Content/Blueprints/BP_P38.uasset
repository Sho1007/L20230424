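; BP_P38 is a player-controlled plane pawn that flies forward constantly and fires rockets.
; Tick feeds the forward vector, scaled by MovementSpeed, into movement input.
; IA_Rotate applies local roll and pitch scaled by delta time and per-axis speeds, steering the flight direction.
; IA_Attack spawns a BP_Rocket at the Arrow component's transform and sets its projectile velocity along the rocket's forward vector.
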(event Input|EnhancedActionEvents|EnhancedInputActionIA_Rotate
  (params (ActionValue :type Vector%202D%20Structure) (ElapsedSeconds :type Float%20%28double-precision%29) (TriggeredSeconds :type Float%20%28double-precision%29) (InputAction :type Input%20Action%20Object%20Reference :default "/Game/Input/IA_Rotate.IA_Rotate"))
  (:Triggered
    (Transformation|AddActorLocalRotation (Math|Rotator|MakeRotator (* (.x ActionValue) (Utilities|Time|GetWorldDeltaSeconds) (Variables|Default|GetRollRotateSpeed)) 0.0 0.0) false false)
    (Transformation|AddActorLocalRotation (Math|Rotator|MakeRotator 0.0 (* (.y ActionValue) (Utilities|Time|GetWorldDeltaSeconds) (Variables|Default|GetPitchRotateSpeed)) 0.0) false false)))

(event Input|EnhancedActionEvents|EnhancedInputActionIA_Attack
  (params (ActionValue :type Boolean) (ElapsedSeconds :type Float%20%28double-precision%29) (TriggeredSeconds :type Float%20%28double-precision%29) (InputAction :type Input%20Action%20Object%20Reference :default "/Game/Input/IA_Attack.IA_Attack"))
  (:Started
    (bind _returnvalue (Game|SpawnActorfromClass "/Game/Blueprints/BP_Rocket.BP_Rocket_C" (Transformation|GetWorldTransform (Variables|Default|GetArrow)) "AlwaysSpawn" 0 0))
    (Variables|/Script/Engine.MovementComponent|SetVelocity (Variables|/Game/Blueprints/BP_Rocket.BP_Rocket_C|GetProjectileMovement _returnvalue) (* (Transformation|GetActorForwardVector _returnvalue) 3e+03))))

(event EventBeginPlay)

(event Collision|EventActorBeginOverlap
  (params (OtherActor :type Actor%20Object%20Reference)))

(event EventTick
  (params (DeltaSeconds :type Float%20%28single-precision%29))
  (Pawn|Input|AddMovementInput (* (Transformation|GetActorForwardVector) (Variables|Default|GetMovementSpeed)) 1.0 false))

(fn ConstructionScript)